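; Grenade pawn or actor that explodes on a one-second fuse started at BeginPlay.
; When the timer fires, it spawns an Explosion actor at its static mesh's transform, plays a 2D explosion sound and destroys itself.
; Until then, a looping Delay entered from Tick toggles the point light's visibility to make it blink.
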(event Custom|Detonate
  (Game|SpawnActorfromClass "/Game/Blueprints/Pawns/Explosion.Explosion_C" (Transformation|GetWorldTransform (Variables|Default|GetStaticMesh)) "Undefined" 0 0)
  (Audio|PlaySound2D "/Game/Effects/Misc/587183__derplayer__explosion-03.587183__derplayer__explosion-03" 1.0 1.0 0.0 0 0)
  (Actor|DestroyActor))

(event Collision|EventActorBeginOverlap
  (params (OtherActor :type Actor%20Object%20Reference)))

(event EventTick
  (params (DeltaSeconds :type Float%20%28single-precision%29))
  (Utilities|FlowControl|Delay 0.3 :!label _label)
  (Rendering|ToggleVisibility (Variables|Default|GetPointLight) false)
  (goto _label))

(event EventBeginPlay
  (Utilities|Time|SetTimerbyEvent (delegate Custom|Detonate) 1.0))

(fn ConstructionScript)