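; Grenade actor that explodes on a short fixed fuse after it spawns.
; BeginPlay starts a one-shot timer that calls Detonate, which spawns an Explosion actor at the grenade's transform and destroys the grenade.
; An unconnected leftover chain with impulse, delay, particle and sound nodes never runs.
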(event Custom|Detonate
  (Game|SpawnActorfromClass "/Game/Blueprints/Pawns/Explosion.Explosion_C" (Transformation|GetActorTransform) "Undefined" 0 0)
  (Actor|DestroyActor))

(event EventBeginPlay
  (Utilities|Time|SetTimerbyEvent (delegate Custom|Detonate) 1.0))

(event Collision|EventActorBeginOverlap
  (params (OtherActor :type Actor%20Object%20Reference)))

(event EventTick
  (params (DeltaSeconds :type Float%20%28single-precision%29)))

(fn ConstructionScript)